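; Enemy1_BP is an enemy actor Blueprint that periodically triggers a combat stance in its animation.
; Each tick feeds delta time into a custom tick event that accumulates a timer, initialized on BeginPlay.
; When the timer passes a fixed threshold of several seconds, it resets and sets CombatStance on the skeletal mesh's Enemy1_AnimBP instance.
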(event Custom|Tick_01
  (params (DeltaInSeconds :type Float%20%28single-precision%29))
  (bind _output_get (Variables|Default|SetTimer (+ DeltaInSeconds (Variables|Default|GetTimer))))
  (if (> _output_get 8.0)
    (Variables|Default|SetTimer 0.0)
    (bind _asenemy_1_anim_bp (Utilities|Casting|CastToEnemy1_AnimBP (Components|SkeletalMesh|GetAnimInstance (Variables|Default|GetSkeletalMesh))))
    (Variables|/Game/Actors/Enemy1/Enemy1_AnimBP.Enemy1_AnimBP_C|SetCombatStance _asenemy_1_anim_bp 1)))

(event EventBeginPlay
  (Variables|Default|SetTimer 0.0))

(event Collision|EventActorBeginOverlap
  (params (OtherActor :type Actor%20Object%20Reference)))

(event EventTick
  (params (DeltaSeconds :type Float%20%28single-precision%29))
  (CallFunction|Tick01 DeltaSeconds))

(fn ConstructionScript)